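; CollectibleRifle_BP is a weapon pickup that equips the player-controlled ALS character that overlaps it.
; A Weapon enum value keys a row in Weapons_DT, whose mesh the construction script applies to the pickup.
; On overlap, that row becomes the character's CurrentWeapon, the held object updates, and the overlay state follows the row's TwoHanded flag.
; DestroyActor is disconnected, so the pickup stays in the level.
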(event EventBeginPlay)

(event Collision|EventActorBeginOverlap
  (params (OtherActor :type Actor%20Object%20Reference))
  (bind _asals_anim_man_character_bp (Utilities|Casting|CastToALS_AnimMan_CharacterBP OtherActor))
  (if (Pawn|IsPlayerControlled _asals_anim_man_character_bp)
    (bind _returnvalue (Utilities|GetDataTableRow "/Game/CustomWeaponSystem/Weapons_DT.Weapons_DT" (Utilities|String|StringToName (Utilities|String|EnumtoString (Variables|Default|GetWeapon))))
      (:then
        (Variables|/Game/AdvancedLocomotionV4/Blueprints/CharacterLogic/ALS_AnimMan_CharacterBP.ALS_AnimMan_CharacterBP_C|SetCurrentWeapon _asals_anim_man_character_bp _returnvalue)
        (Default|UpdateHeldObject _asals_anim_man_character_bp)
        (Class|ALSCharacterBPI|BPISetOverlayState(Message) _asals_anim_man_character_bp (select (.TwoHanded (Utilities|Struct|BreakWeapon _returnvalue)) "NewEnumerator1" "NewEnumerator10"))))))

(event EventTick
  (params (DeltaSeconds :type Float%20%28single-precision%29)))

(fn ConstructionScript
  (bind _weapon (Variables|Default|GetWeapon))
  (bind _returnvalue (Utilities|String|EnumtoString _weapon))
  (bind _returnvalue_2 (Utilities|String|StringToName _returnvalue))
  (bind _returnvalue_3 (Utilities|GetDataTableRow "/Game/CustomWeaponSystem/Weapons_DT.Weapons_DT" _returnvalue_2)
    (:then
      (Development|PrintString _returnvalue)
      (Components|SkeletalMesh|SetSkeletalMeshAsset (Variables|Default|GetSkeletalMesh) (.mesh _returnvalue_3)))
    (:RowNotFound
      (Development|PrintString (Utilities|String|Append "Row " (Utilities|String|ToString(Name) _returnvalue_2) " not found!")))))